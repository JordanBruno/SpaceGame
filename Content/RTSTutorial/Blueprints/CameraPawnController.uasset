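; Controller for an RTS camera pawn that handles forward/back navigation from the MoveForward axis unless DisableCamNav is set.
; BeginPlay caches the player's CameraPawn, and the axis event sets its transform from MovementX, passing a speed derived from clamped spring-arm length and FastMoveMultiplier.
; MovementX holds math for a local-X offset, but those nodes are not wired to any output.
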(event EventBeginPlay
  (Utilities|FlowControl|Sequence
    (:then_0
      (Utilities|ReferenceCasts))))

(event Input|AxisEvents|InputAxisMoveForward
  (params (AxisValue :type Float%20%28single-precision%29))
  (if (not (Variables|Default|GetDisableCamNav))
    (Transformation|SetActorTransform (Variables|References|GetCameraPawnRef) (Utilities|MovementX (CallFunction|MovementSpeedCalculation) (Variables|Default|GetFastMoveMultiplier) AxisValue (Variables|References|GetCameraPawnRef)))))

(fn ConstructionScript)

(fn MovementSpeedCalculation
  (return (Math|Float|Clamp(Float) (/ (Variables|/Script/Engine.SpringArmComponent|GetTargetArmLength (Variables|/Game/RTSTutorial/Blueprints/CameraPawn.CameraPawn_C|GetSpringArm (Variables|References|GetCameraPawnRef))) 1e+02) 5.0 2e+01)))